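; BP_PressureTrigger is an actionable pressure trigger that signals receivers when actors begin or end overlapping it.
; Overlap events fire activated/deactivated dispatchers and swap the static mesh material between check and disabled looks.
; Interface events forward receiver delegates to those dispatchers for binding and unbinding.
; Overlaps are neither filtered nor counted, so any exit deactivates it, and GetState always returns false.
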(event `self.ReceiveActorBeginOverlap`
  (params (OtherActor :type "Actor Object Reference"))
  ;[0.6403 0.4605 1] Actionable State Detection
  (`self.OnActivated`)
  (`self.LocalOnActivated`))

(event `self.ReceiveActorEndOverlap`
  (params (OtherActor :type "Actor Object Reference"))
  ;[0.6403 0.4605 1] Actionable State Detection
  (`self.OnDeactivated`)
  (`self.LocalOnDeactivated`))

(event `self.BindEventToOnActivated`
  (params (Delegate :type "Delegate (by ref)"))
  ;[0.5214 1 0.4071] Interface Binding For Receivers
  (add `self.OnActivated` Delegate))

(event `self.UnbindEventFromOnActivated`
  (params (Delegate :type "Delegate (by ref)"))
  ;[0.5214 1 0.4071] Interface Binding For Receivers
  (remove `self.OnActivated` Delegate))

(event `self.BindEventToOnDeactivated`
  (params (Delegate :type "Delegate (by ref)"))
  ;[0.5214 1 0.4071] Interface Binding For Receivers
  (add `self.OnDeactivated` Delegate))

(event `self.UnbindEventFromOnDeactivated`
  (params (Delegate :type "Delegate (by ref)"))
  ;[0.5214 1 0.4071] Interface Binding For Receivers
  (remove `self.OnDeactivated` Delegate))

(fn `GetState`
  (returns (ReturnValue :type Boolean))
  (return false))

(fn `LocalOnActivated`
  (`PrimitiveComponent.SetMaterial` (`self.StaticMesh`) 0 "/Engine/EditorMaterials/CheckMaterial.CheckMaterial"))

(fn `LocalOnDeactivated`
  (`PrimitiveComponent.SetMaterial` (`self.StaticMesh`) 0 "/Engine/EditorMaterials/Cascade/CASC_ModuleDisable_MAT.CASC_ModuleDisable_MAT"))

(fn `UserConstructionScript`)