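; Cable prop that follows a spline and changes its material to show whether its linked Actionable is active.
; The construction script adds a Z-forward spline mesh component for each spline point and stores them in an array.
; On BeginPlay it binds to the Actionable's activated and deactivated messages through the Actionable interface.
; Each message swaps the first material slot on every stored segment between two fixed materials.
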(event `self.ReceiveBeginPlay`
  (bind _actionable (`self.Actionable`))
  (if (`KismetSystemLibrary.DoesImplementInterface` _actionable "/Script/cp_rtal.Actionable")
    (`|ExecutionSequence`
      (:`then_0`
        (message `Actionable.BindEventToOnActivated` _actionable (delegate `/Game/Gameplay/Interfaces/Receiver.OnAllActionablesActive`)))
      (:`then_1`
        (message `Actionable.BindEventToOnDeactivated` _actionable (delegate `/Game/Gameplay/Interfaces/Receiver.OnAllActionablesActiveCancelled`))))))

(event `/Game/Gameplay/Interfaces/Receiver.OnAllActionablesActive`
  (`self.PropagateNewMaterial` "/Engine/MapTemplates/Materials/BasicAsset03.BasicAsset03"))

(event `/Game/Gameplay/Interfaces/Receiver.OnAllActionablesActiveCancelled`
  (`self.PropagateNewMaterial` "/Engine/EditorMaterials/Camera/CineMat.CineMat"))

(fn `PropagateNewMaterial`
  (params (NewParam :type "Material Object Reference"))
  (for _array_element (`self.Meshes`)
    (`PrimitiveComponent.SetMaterial` _array_element 0 NewParam)))

(fn `UserConstructionScript`
  (bind _spline (`self.Spline`))
  (for _index (range (`SplineComponent.GetNumberOfSplinePoints` (`self.Spline`)))
    (bind _returnvalue (`AddComponent|NODE_AddSplineMeshComponent-1`))
    (`SplineMeshComponent.SetForwardAxis` _returnvalue "Z" true)
    (bind _returnvalue_2 (+ _index 1))
    (`SplineMeshComponent.SetStartAndEnd` _returnvalue (`SplineComponent.GetLocationAtSplinePoint` _spline _index "Local") (`SplineComponent.GetTangentAtSplinePoint` _spline _index "Local") (`SplineComponent.GetLocationAtSplinePoint` _spline _returnvalue_2 "Local") (`SplineComponent.GetTangentAtSplinePoint` _spline _returnvalue_2 "Local") true)
    (`KismetArrayLibrary.Array_Append` (`self.Meshes`) (`|MakeArray` _returnvalue))))