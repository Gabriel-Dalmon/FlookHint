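; Respawn checkpoint that registers itself as the active one on the Cubot player controller when the player's character overlaps it.
; It deactivates the previous checkpoint, swaps its cube material and stores a copy of the character's carried item as a backup.
; Deactivation restores the disabled material and destroys the backup item.
; IsActive is never set true, and Activate destroys the checkpoint itself when a backup already exists.
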(event `self.ReceiveBeginPlay`
  (set `self.IsActive` false))

(event `self.ReceiveActorBeginOverlap`
  (params (OtherActor :type "Actor Object Reference"))
  (if (not (`self.IsActive`))
    ;[1 1 1] Is Player
    (bind _asbp_cubot_character (cast `/Game/Core/CharacterController/BP_CubotCharacter` OtherActor))
    (bind _asbp_cubot_controller (cast `/Game/Core/CharacterController/BP_CubotController` (`Pawn.GetController` _asbp_cubot_character)))
    (bind _activerespawncheckpoint (`/Game/Core/CharacterController/BP_CubotController.ActiveRespawnCheckpoint` _asbp_cubot_controller))
    ;[1 1 1] Update Checkpoint
    (`/Engine/EditorBlueprintResources/StandardMacros.IsValid` _activerespawncheckpoint
      (:`Is Valid`
        (`self.Deactivate` _activerespawncheckpoint))
      (:`Is Not Valid`
        _))
    (set `/Game/Core/CharacterController/BP_CubotController.ActiveRespawnCheckpoint` self _asbp_cubot_controller)
    (`self.Activate` _asbp_cubot_character)))

(fn `Activate`
  (params (Character :type "/Game/Core/CharacterController/BP_CubotCharacter Object Reference"))
  (bind _carrieditem (`/Game/Core/CharacterController/BP_CubotCharacter.CarriedItem` Character))
  (`/Engine/EditorBlueprintResources/StandardMacros.IsValid` (`self.BackupItem`)
    (:`Is Valid`
      (`self.K2_DestroyActor`))
    (:`Is Not Valid`
      _))
  (`/Engine/EditorBlueprintResources/StandardMacros.IsValid` _carrieditem
    (:`Is Valid`
      (bind _copy (`/Game/Blueprints/Items/BP_Item.CopyFromActor` _carrieditem))
      (set `self.BackupItem` _copy))
    (:`Is Not Valid`
      _))
  (`PrimitiveComponent.SetMaterial` (`self.Cube`) 0 "/Engine/EditorMaterials/CheckMaterial.CheckMaterial"))

(fn `Deactivate`
  (bind _backupitem (`self.BackupItem`))
  (`PrimitiveComponent.SetMaterial` (`self.Cube`) 0 "/Engine/EditorMaterials/Cascade/CASC_ModuleDisable_MAT.CASC_ModuleDisable_MAT")
  (`/Engine/EditorBlueprintResources/StandardMacros.IsValid` _backupitem
    (:`Is Valid`
      (`self.K2_DestroyActor` _backupitem))))

(fn `UserConstructionScript`)