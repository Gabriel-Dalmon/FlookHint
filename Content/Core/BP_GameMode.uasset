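; Game mode that handles respawning the player as a new Cubot character at the active checkpoint.
; The respawn event spawns and possesses the character at the checkpoint's spawn point, or reloads the current level without a valid checkpoint.
; Any backup item stored on the checkpoint is attached to the new character, a copy is stored back for later respawns, and the gun input mapping is added.
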(event `Respawn Player_Event`
  (params (`Player Controller` :type "/Game/Core/CharacterController/BP_CubotController Object Reference") (HasPortalGun :type Boolean))
  (bind _backupitem (`self.BackupItem`))
  (bind _activerespawncheckpoint (`/Game/Core/CharacterController/BP_CubotController.ActiveRespawnCheckpoint` `Player Controller`))
  ;[0.2663 1 0.2359] Respawn Logic
  (`/Engine/EditorBlueprintResources/StandardMacros.IsValid` _activerespawncheckpoint
    (:`Is Valid`
      (set `self.BackupItem` (`/Game/Environment/BP_RespawnCheckpoint.BackupItem` _activerespawncheckpoint))
      (set `/Game/Environment/BP_RespawnCheckpoint.BackupItem` null _activerespawncheckpoint)
      (bind _returnvalue (`|SpawnActorFromClass` "/Game/Core/CharacterController/BP_CubotCharacter.BP_CubotCharacter_C" (`SceneComponent.K2_GetComponentToWorld` (`/Game/Environment/BP_RespawnCheckpoint.SpawnPoint` _activerespawncheckpoint)) "AlwaysSpawn" "MultiplyWithRoot" null null))
      (`Controller.Possess` `Player Controller` _returnvalue)
      ;;[1 1 1] Should be encapsulated elsewhere
      (`/Engine/EditorBlueprintResources/StandardMacros.IsValid` (`self.BackupItem`)
        (:`Is Valid`
          (bind _returnvalue_2 (`self.K2_AttachToComponent` (`self.BackupItem`) (`/Game/Core/CharacterController/BP_CubotCharacter.ItemSocket` _returnvalue) "None" "KeepRelative" "KeepRelative" "KeepRelative" true))
          (if _returnvalue_2
            (`self.SetActorHiddenInGame` _backupitem false)
            (set `/Game/Core/CharacterController/BP_CubotCharacter.CarriedItem` _backupitem _returnvalue)
            (bind _copy (`/Game/Blueprints/Items/BP_Item.CopyFromActor` _backupitem))
            (set `/Game/Environment/BP_RespawnCheckpoint.BackupItem` _copy _activerespawncheckpoint)
            (`self.SetOwner` _backupitem _returnvalue))
          (`EnhancedInputSubsystemInterface.AddMappingContext` (pcsubsystem `EnhancedInputLocalPlayerSubsystem` (`GameplayStatics.GetPlayerController` 0)) "/Game/Inputs/GunInputMapping.GunInputMapping" 0 (struct))
          (set `self.BackupItem` null))))
    (:`Is Not Valid`
      (bind _returnvalue_3 (`GameplayStatics.GetCurrentLevelName` true))
      (`GameplayStatics.OpenLevel` (`KismetStringLibrary.Conv_StringToName` _returnvalue_3)))))

(fn `UserConstructionScript`)