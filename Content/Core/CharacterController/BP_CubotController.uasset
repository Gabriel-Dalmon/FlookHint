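; Player controller for Cubot that maps Enhanced Input to the player pawn and handles death and respawn.
; BeginPlay adds the mapping context, and input actions drive movement, look, jump, the character's lamp and the pause menu.
; On possession it binds to the Cubot's HealthComponent death event.
; Death destroys the pawn and asks BP_GameMode to respawn it, with the portal gun flag hard-coded to true.
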(event `self.ReceiveBeginPlay`
  ;[0.5379 1 0.1754] Initialization
  (`EnhancedInputSubsystemInterface.AddMappingContext` (pcsubsystem `EnhancedInputLocalPlayerSubsystem` self) "/Game/Inputs/CubotInputMappingContext.CubotInputMappingContext" 0 (struct)))

(event `EnhancedInput|/Game/Inputs/IA_Jump`
  (params (ActionValue :type Boolean) (ElapsedSeconds :type "Float (double-precision)") (TriggeredSeconds :type "Float (double-precision)") (InputAction :type "InputAction Object Reference" :default "/Game/Inputs/IA_Jump.IA_Jump"))
  ;[1 1 1] Jump Mapping
  (:`Triggered`
    (bind _ascharacter (cast `Character` (`GameplayStatics.GetPlayerPawn` 0)))
    (`Character.Jump` _ascharacter)))

(event `EnhancedInput|/Game/Inputs/IA_TernaryInteract`
  (params (ActionValue :type Boolean) (ElapsedSeconds :type "Float (double-precision)") (TriggeredSeconds :type "Float (double-precision)") (InputAction :type "InputAction Object Reference" :default "/Game/Inputs/IA_TernaryInteract.IA_TernaryInteract"))
  ;[1 1 1] Interaction2 Mapping
  (:`Triggered`
    (bind _ascubot_character (cast `CubotCharacter` (`GameplayStatics.GetPlayerPawn` 0)))
    (`CubotCharacter.TurnOnLamp` _ascubot_character)))

(event `EnhancedInput|/Game/Inputs/IA_Move`
  (params (ActionValue :type "Vector2D Structure") (ElapsedSeconds :type "Float (double-precision)") (TriggeredSeconds :type "Float (double-precision)") (InputAction :type "InputAction Object Reference" :default "/Game/Inputs/IA_Move.IA_Move"))
  ;[1 1 1] Movement Mapping
  (:`Triggered`
    (bind _ascharacter (cast `Character` (`GameplayStatics.GetPlayerPawn` 0)))
    (`Pawn.AddMovementInput` _ascharacter (`self.GetActorRightVector` _ascharacter) ActionValue_X false)
    (`Pawn.AddMovementInput` _ascharacter (`self.GetActorForwardVector` _ascharacter) ActionValue_Y false)))

(event `EnhancedInput|/Game/Inputs/IA_Look`
  (params (ActionValue :type "Vector2D Structure") (ElapsedSeconds :type "Float (double-precision)") (TriggeredSeconds :type "Float (double-precision)") (InputAction :type "InputAction Object Reference" :default "/Game/Inputs/IA_Look.IA_Look"))
  ;[1 1 1] Look Mapping
  (:`Triggered`
    (bind _ascharacter (cast `Character` (`GameplayStatics.GetPlayerPawn` 0)))
    (`Pawn.AddControllerYawInput` _ascharacter ActionValue_X)
    (`Pawn.AddControllerPitchInput` _ascharacter ActionValue_Y)))

(event `self.ReceivePossess`
  (params (PossessedPawn :type "Pawn Object Reference"))
  ;[1 0.1302 0.1302] Death Logic
  (bind _ascubot_character (cast `CubotCharacter` PossessedPawn))
  (add `HealthComponent.OnDeadEvent` (`CubotCharacter.HealthComponent` _ascubot_character) (delegate `On Character Dead`)))

(event `On Character Dead`
  ;[1 0.1302 0.1302] Death Logic
  (`self.K2_DestroyActor` (`GameplayStatics.GetPlayerPawn` 0))
  (bind _asbase_game_mode (cast `/Game/Core/BP_GameMode` (`GameplayStatics.GetGameMode`)))
  (`/Game/Core/BP_GameMode.Respawn Player_Event` _asbase_game_mode self true) ; Should replace HasPortalGun with get item (but probably needs to be stored before DestroyActor is called)
)

(event `EnhancedInput|/Game/Inputs/IA_PauseGame`
  (params (ActionValue :type Boolean) (ElapsedSeconds :type "Float (double-precision)") (TriggeredSeconds :type "Float (double-precision)") (InputAction :type "InputAction Object Reference" :default "/Game/Inputs/IA_PauseGame.IA_PauseGame"))
  (bind _pausemenu (`self.PauseMenu`))
  (:`Triggered`
    (`/Engine/EditorBlueprintResources/StandardMacros.IsValid` _pausemenu
      (:`Is Valid`
        (bind _asui_pause_menu (cast `/Game/UI/Pages/UI_PauseMenu` _pausemenu)
          (:`then`
            (`/Game/UI/Pages/UI_PauseMenu.Show` _asui_pause_menu))
          (:`CastFailed`
            (bind _returnvalue (`|CreateWidget` "/Game/UI/Pages/UI_PauseMenu.UI_PauseMenu_C" :!label _label))
            (`/Game/UI/Pages/UI_PauseMenu.Show` _returnvalue))))
      (:`Is Not Valid`
        (goto _label)))))

(fn `UserConstructionScript`)