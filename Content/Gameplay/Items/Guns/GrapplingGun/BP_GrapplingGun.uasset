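; Grappling gun item that lets the owning Cubot character attach to a traced point, swing from it and pull on the hook.
; Primary traces from the camera direction and spawns a BP_Hook with a distance-limited physics constraint, or releases it; Secondary toggles pulling.
; While attached, the flying character is teleported to the hook's simulated physics object each tick and the cable follows.
; Release launches the character with that object's velocity.
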(event `self.ReceiveDestroyed`
  (`/Engine/EditorBlueprintResources/StandardMacros.IsValid` (`self.Hook`)
    (:`Is Valid`
      (`self.K2_DestroyActor` (`self.Hook`)))))

(event `self.ReceiveTick`
  (params (DeltaSeconds :type "Float (single-precision)"))
  (if (`self.IsAttached`)
    (set `CableComponent.EndLocation` (`KismetMathLibrary.InverseTransformLocation` (`self.GetTransform`) (`self.AttachPoint`)) (`self.Cable`))
    (`self.K2_SetActorLocation` (`self.GetOwner`) (`SceneComponent.K2_GetComponentLocation` (`/Game/Gameplay/Items/Guns/GrapplingGun/BP_Hook.PhysicsObject` (`self.Hook`))) false true)))

(fn `FindGrapplingPoint`
  (returns (AttachPoint :type "Vector Structure") (AttachActor :type "Actor Object Reference") (HasFoundAttachPoint :type Boolean) (AttachNormal :type "Vector Structure"))
  (bind _returnvalue (`SceneComponent.K2_GetComponentLocation` (`self.Muzzle`)))
  (bind _asbp_cubot_character (cast `/Game/Gameplay/Core/CharacterController/BP_CubotCharacter` (`self.GetOwner`)))
  (bind (_outhit _returnvalue_2) (`KismetSystemLibrary.LineTraceSingle` :`Start` _returnvalue :`End` (+ _returnvalue (* (`KismetMathLibrary.GetForwardVector` (`SceneComponent.K2_GetComponentRotation` (`/Game/Gameplay/Core/CharacterController/BP_CubotCharacter.Camera` _asbp_cubot_character))) (`self.GrapplingRange`))) :`TraceChannel` "TraceTypeQuery1" :`DrawDebugType` "ForDuration"))
  (bind (_bblockinghit _binitialoverlap _time _distance _location _impactpoint _normal _impactnormal _physmat _hitactor) (`GameplayStatics.BreakHitResult` _outhit))
  (return _impactpoint _hitactor _returnvalue_2 _impactnormal))

(fn `OnHookAttached`
  (bind _ascubot_character (cast `CubotCharacter` (`self.GetOwner`)))
  (`CharacterMovementComponent.SetMovementMode` (`Character.CharacterMovement` _ascubot_character) "MOVE_Flying" 0)
  (`self.OnHookUpdated` true))

(fn `OnHookReleased`
  (bind _ascubot_character (cast `CubotCharacter` (`self.GetOwner`)))
  (`CharacterMovementComponent.SetMovementMode` (`Character.CharacterMovement` _ascubot_character) "MOVE_Falling" 0)
  (`self.OnHookUpdated` false)
  (set `self.IsPulling` false)
  (bind _asbp_cubot_character (cast `/Game/Gameplay/Core/CharacterController/BP_CubotCharacter` (`self.GetOwner`)))
  (`Character.LaunchCharacter` _asbp_cubot_character (`SceneComponent.GetComponentVelocity` (`/Game/Gameplay/Items/Guns/GrapplingGun/BP_Hook.PhysicsObject` (`self.Hook`))) true true)
  (`self.K2_DestroyActor` (`self.Hook`)))

(fn `OnHookUpdated`
  (params (IsAttached :type Boolean))
  (set `self.IsAttached` IsAttached)
  (`SceneComponent.SetVisibility` (`self.Cable`) IsAttached false))

(fn `OnInteractBegin`
  (params (InteractionType :type "/Game/Inputs/EInteractionTypes Enum" :default "NewEnumerator0"))
  (bind _hook (`self.Hook`))
  (`parent.OnInteractBegin` InteractionType)
  (switch `/Game/Inputs/EInteractionTypes` InteractionType
    (:`NewEnumerator0`
      (if (`self.IsAttached`)
        (`self.OnHookReleased`)
        (else
          (`self.TryAttachHook`))))
    (:`NewEnumerator1`
      (if (`self.IsAttached`)
        (set `self.IsPulling` true)
        (set `/Game/Gameplay/Items/Guns/GrapplingGun/BP_Hook.IsPulling` true _hook)
        (`/Game/Gameplay/Items/Guns/GrapplingGun/BP_Hook.OnPulled` _hook)))))

(fn `OnInteractEnd`
  (params (InteractionType :type "/Game/Inputs/EInteractionTypes Enum" :default "NewEnumerator0"))
  (`parent.OnInteractEnd` InteractionType)
  (switch `/Game/Inputs/EInteractionTypes` InteractionType
    (:`NewEnumerator1`
      (if (`self.IsAttached`)
        (set `self.IsPulling` false)
        (set `/Game/Gameplay/Items/Guns/GrapplingGun/BP_Hook.IsPulling` false (`self.Hook`))))))

(fn `TryAttachHook`
  (bind _returnvalue (`self.GetOwner`))
  (bind _returnvalue_2 (`self.K2_GetActorLocation` _returnvalue))
  (bind (_attachpoint _attachactor _hasfoundattachpoint _attachnormal) (`self.FindGrapplingPoint`))
  (if _hasfoundattachpoint
    (if (`self.IsActorAttachable` _attachactor)
      (set `self.AttachPoint` _attachpoint)
      (bind _returnvalue_3 (`|SpawnActorFromClass` "/Game/Gameplay/Items/Guns/GrapplingGun/BP_Hook.BP_Hook_C" (`KismetMathLibrary.MakeTransform` _attachpoint (struct :`Pitch` 180.0)) "AlwaysSpawn" "MultiplyWithRoot" null null))
      (bind _output_get (set `self.Hook` _returnvalue_3))
      (bind _returnvalue_4 (`PhysicsConstraintComponent.GetConstraint` (`/Game/Gameplay/Items/Guns/GrapplingGun/BP_Hook.PhysicsConstraint` _output_get)))
      (`ConstraintInstanceBlueprintLibrary.SetLinearLimits` _returnvalue_4 "LCM_Limited" "LCM_Limited" "LCM_Limited" (`KismetMathLibrary.Vector_Distance` _returnvalue_2 _attachpoint))
      (bind _physicsobject (`/Game/Gameplay/Items/Guns/GrapplingGun/BP_Hook.PhysicsObject` _output_get))
      (`SceneComponent.K2_SetWorldTransform` _physicsobject (`KismetMathLibrary.MakeTransform` _returnvalue_2 (struct :`Pitch` 180.0)) false true)
      (`PrimitiveComponent.SetPhysicsLinearVelocity` _physicsobject (`self.GetVelocity` _returnvalue) false "None")
      (`self.OnHookAttached`))))

(fn `UserConstructionScript`)