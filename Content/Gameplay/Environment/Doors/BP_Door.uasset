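; BP_Door is a double sliding door that opens when all of its linked Actionables are active.
; BeginPlay sets the animation speed and binds to activation and deactivation messages of each entry implementing the Actionable interface.
; A counter of active entries triggers opening at the full count, and closing when it drops to one below full or to zero.
; One timeline slides both panels along X, played in reverse to close.
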(event `Open_Event`
  (bind (_direction _rightdoorx _leftdoorx) (`Timeline|Timeline` :!label _label)
    (:`Update`
      (`|ExecutionSequence`
        (:`then_0`
          (`SceneComponent.K2_SetRelativeLocation` (`self.RightDoor`) (`KismetMathLibrary.MakeVector` _rightdoorx) false false))
        (:`then_1`
          (`SceneComponent.K2_SetRelativeLocation` (`self.LeftDoor`) (`KismetMathLibrary.MakeVector` _leftdoorx) false false))))))

(event `Close_Event`
  (goto _label :!via `Reverse`))

(event `self.ReceiveBeginPlay`
  (`TimelineComponent.SetPlayRate` (`self.Timeline`) (`self.DoorAnimationSpeed`))
  (for _array_element (`self.Actionables`)
    (if (`KismetSystemLibrary.DoesImplementInterface` _array_element "/Script/cp_rtal.Actionable")
      (`|ExecutionSequence`
        (:`then_0`
          (message `Actionable.BindEventToOnActivated` _array_element (delegate `/Game/Gameplay/Interfaces/Receiver.OnSingleActionableActivated`)))
        (:`then_1`
          (message `Actionable.BindEventToOnDeactivated` _array_element (delegate `/Game/Gameplay/Interfaces/Receiver.OnSingleActionableDeactivated`)))))))

(event `/Game/Gameplay/Interfaces/Receiver.OnSingleActionableActivated`
  (set `self.activeActionablesCount` (+ (`self.activeActionablesCount`) 1))
  (if (>= (`self.activeActionablesCount`) (`KismetArrayLibrary.Array_Length` (`self.Actionables`)))
    (`self.OnAllActionablesActive`)))

(event `/Game/Gameplay/Interfaces/Receiver.OnSingleActionableDeactivated`
  (bind _activeactionablescount (`self.activeActionablesCount`))
  (set `self.activeActionablesCount` (- (`self.activeActionablesCount`) 1))
  (if (or (== _activeactionablescount 0) (== _activeactionablescount (- (`KismetArrayLibrary.Array_Length` (`self.Actionables`)) 1)))
    (`self.OnAllActionablesActiveCancelled`)))

(event `/Game/Gameplay/Interfaces/Receiver.OnAllActionablesActiveCancelled`
  (`self.Close_Event`))

(event `/Game/Gameplay/Interfaces/Receiver.OnAllActionablesActive`
  (`self.Open_Event`))

(fn `UserConstructionScript`)