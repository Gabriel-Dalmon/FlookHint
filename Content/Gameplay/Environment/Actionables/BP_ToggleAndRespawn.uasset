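; BP_ToggleAndRespawn is an actionable respawn checkpoint that doubles as a one-way trigger.
; When inactive and overlapped by the Cubot player, it deactivates the controller's previous checkpoint, registers itself and calls Activate; Deactivate destroys BackupItem.
; Separately, the first overlap by any actor notifies bound receivers and swaps the cube material.
; The deactivation notification is unwired, and GetState always returns false.
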(event `self.ReceiveActorBeginOverlap`
  (params (OtherActor :type "Actor Object Reference"))
  ;[0.6403 0.4605 1] Actionable State Detection
  (`|ExecutionSequence`
    (:`then_0`
      (if (not (`self.IsActive`))
        ;[1 1 1] Is Player
        (bind _asbp_cubot_character (cast `/Game/Gameplay/Core/CharacterController/BP_CubotCharacter` OtherActor))
        (bind _asbp_cubot_controller (cast `/Game/Gameplay/Core/CharacterController/BP_CubotController` (`Pawn.GetController` _asbp_cubot_character)))
        (bind _activerespawncheckpoint (`/Game/Gameplay/Core/CharacterController/BP_CubotController.ActiveRespawnCheckpoint` _asbp_cubot_controller))
        ;[1 1 1] Update Checkpoint
        (`/Engine/EditorBlueprintResources/StandardMacros.IsValid` _activerespawncheckpoint
          (:`Is Valid`
            (`self.Deactivate` _activerespawncheckpoint))
          (:`Is Not Valid`
            _))
        (set `/Game/Gameplay/Core/CharacterController/BP_CubotController.ActiveRespawnCheckpoint` self _asbp_cubot_controller)
        (`self.Activate` _asbp_cubot_character)))
    (:`then_1`
      (if (not (`self.IsActivated`))
        (`self.OnActivated`)
        (`self.LocalOnActivated`)
        (set `self.IsActivated` true)))))

(event `self.BindEventToOnActivated`
  (params (Delegate :type "Delegate (by ref)"))
  ;[0.5214 1 0.4071] Interface Binding For Receivers
  (add `self.OnActivated` Delegate))

(event `self.UnbindEventFromOnActivated`
  (params (Delegate :type "Delegate (by ref)"))
  ;[0.5214 1 0.4071] Interface Binding For Receivers
  (remove `self.OnActivated` Delegate))

(event `self.BindEventToOnDeactivated`
  (params (Delegate :type "Delegate (by ref)"))
  ;[0.5214 1 0.4071] Interface Binding For Receivers
  (add `self.OnDeactivated` Delegate))

(event `self.UnbindEventFromOnDeactivated`
  (params (Delegate :type "Delegate (by ref)"))
  ;[0.5214 1 0.4071] Interface Binding For Receivers
  (remove `self.OnDeactivated` Delegate))

(fn `Deactivate`
  (bind _backupitem (`self.BackupItem`))
  (`/Engine/EditorBlueprintResources/StandardMacros.IsValid` _backupitem
    (:`Is Valid`
      (`self.K2_DestroyActor` _backupitem))))

(fn `GetState`
  (returns (ReturnValue :type Boolean))
  (return false))

(fn `LocalOnActivated`
  (`PrimitiveComponent.SetMaterial` (`self.Cube`) 0 "/Engine/EditorMaterials/CheckMaterial.CheckMaterial"))

(fn `LocalOnDeactivated`
  (`PrimitiveComponent.SetMaterial` (`self.Cube`) 0 "/Engine/EditorMaterials/Cascade/CASC_ModuleDisable_MAT.CASC_ModuleDisable_MAT"))

(fn `UserConstructionScript`)