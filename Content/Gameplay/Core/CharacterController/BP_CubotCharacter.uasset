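; BP_CubotCharacter is the Cubot character Blueprint, which manages the item the character carries.
; Enhanced Input actions for primary, secondary and ternary interaction forward to the valid CarriedItem's OnInteractBegin, each with its own enum value.
; Only secondary interaction also calls OnInteractEnd, on either cancel or completion.
; When the character is destroyed, it destroys its carried item too.
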(event `self.ReceiveDestroyed`
  ; Manage Carried Item
  (`/Engine/EditorBlueprintResources/StandardMacros.IsValid` (`self.CarriedItem`)
    (:`Is Valid`
      (`self.K2_DestroyActor` (`self.CarriedItem`)))))

(event `EnhancedInput|/Game/Inputs/IA_PrimaryInteract`
  (params (ActionValue :type Boolean) (ElapsedSeconds :type "Float (double-precision)") (TriggeredSeconds :type "Float (double-precision)") (InputAction :type "InputAction Object Reference" :default "/Game/Inputs/IA_PrimaryInteract.IA_PrimaryInteract"))
  ; Manage Carried Item
  (:`Started`
    (`/Engine/EditorBlueprintResources/StandardMacros.IsValid` (`self.CarriedItem`)
      (:`Is Valid`
        (`/Game/Gameplay/Items/BP_Item.OnInteractBegin` (`self.CarriedItem`) "NewEnumerator0")))))

(event `EnhancedInput|/Game/Inputs/IA_SecondaryInteract`
  (params (ActionValue :type Boolean) (ElapsedSeconds :type "Float (double-precision)") (TriggeredSeconds :type "Float (double-precision)") (InputAction :type "InputAction Object Reference" :default "/Game/Inputs/IA_SecondaryInteract.IA_SecondaryInteract"))
  ; Manage Carried Item
  (:`Started`
    (`/Engine/EditorBlueprintResources/StandardMacros.IsValid` (`self.CarriedItem`)
      (:`Is Valid`
        (`/Game/Gameplay/Items/BP_Item.OnInteractBegin` (`self.CarriedItem`) "NewEnumerator1"))))
  (:`Canceled`
    (`/Engine/EditorBlueprintResources/StandardMacros.IsValid` (`self.CarriedItem`) :!label _label
      (:`Is Valid`
        (`/Game/Gameplay/Items/BP_Item.OnInteractEnd` (`self.CarriedItem`) "NewEnumerator1"))))
  (:`Completed`
    (goto _label)))

(event `EnhancedInput|/Game/Inputs/IA_TernaryInteract`
  (params (ActionValue :type Boolean) (ElapsedSeconds :type "Float (double-precision)") (TriggeredSeconds :type "Float (double-precision)") (InputAction :type "InputAction Object Reference" :default "/Game/Inputs/IA_TernaryInteract.IA_TernaryInteract"))
  ; Manage Carried Item
  (:`Triggered`
    (`/Engine/EditorBlueprintResources/StandardMacros.IsValid` (`self.CarriedItem`)
      (:`Is Valid`
        (`/Game/Gameplay/Items/BP_Item.OnInteractBegin` (`self.CarriedItem`) "NewEnumerator2")))))

(fn `UserConstructionScript`)