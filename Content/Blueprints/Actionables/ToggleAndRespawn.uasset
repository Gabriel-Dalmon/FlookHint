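; Actionable toggle that doubles as a respawn checkpoint, activated when an actor overlaps it while it is inactive.
; Activation notifies bound receivers and swaps the mesh to the check material.
; For a Cubot player, it registers as the controller's checkpoint only if none is valid, saving the carried item's class.
; Interface events expose delegate binding; deactivation logic is unwired and GetState always returns false.
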(event `self.ReceiveActorBeginOverlap`
  (params (OtherActor :type "Actor Object Reference"))
  ;[0.6403 0.4605 1] Actionable State Detection
  (if (not (`self.IsActivated`))
    (`self.OnActivated`)
    (`self.LocalOnActivated`)
    ;[1 1 1] Is Player
    (bind _asbp_cubot_character (cast `/Game/Blueprints/CharacterController/BP_CubotCharacter` OtherActor))
    (bind _asbp_cubot_controller (cast `/Game/Blueprints/CharacterController/BP_CubotController` (`Pawn.GetController` _asbp_cubot_character)))
    ;[1 1 1] Update Checkpoint
    (`/Engine/EditorBlueprintResources/StandardMacros.IsValid` (`/Game/Blueprints/CharacterController/BP_CubotController.ActiveRespawnCheckpoint` _asbp_cubot_controller)
      (:`Is Not Valid`
        (set `/Game/Blueprints/CharacterController/BP_CubotController.ActiveRespawnCheckpoint` self _asbp_cubot_controller)
        (set `self.CarriedItem` (`GameplayStatics.GetObjectClass` (`/Game/Blueprints/CharacterController/BP_CubotCharacter.CarriedItem` _asbp_cubot_character)))))))

(event `self.BindEventToOnActivated`
  (params (Delegate :type "Delegate (by ref)"))
  ;[0.5214 1 0.4071] Interface Binding For Receivers
  (add `self.OnActivated` Delegate))

(event `self.UnbindEventFromOnActivated`
  (params (Delegate :type "Delegate (by ref)"))
  ;[0.5214 1 0.4071] Interface Binding For Receivers
  (remove `self.OnActivated` Delegate))

(event `self.BindEventToOnDeactivated`
  (params (Delegate :type "Delegate (by ref)"))
  ;[0.5214 1 0.4071] Interface Binding For Receivers
  (add `self.OnDeactivated` Delegate))

(event `self.UnbindEventFromOnDeactivated`
  (params (Delegate :type "Delegate (by ref)"))
  ;[0.5214 1 0.4071] Interface Binding For Receivers
  (remove `self.OnDeactivated` Delegate))

(fn `GetState`
  (returns (ReturnValue :type Boolean))
  (return false))

(fn `LocalOnActivated`
  (`PrimitiveComponent.SetMaterial` (`self.StaticMesh`) 0 "/Engine/EditorMaterials/CheckMaterial.CheckMaterial"))

(fn `LocalOnDeactivated`
  (`PrimitiveComponent.SetMaterial` (`self.StaticMesh`) 0 "/Engine/EditorMaterials/Cascade/CASC_ModuleDisable_MAT.CASC_ModuleDisable_MAT"))

(fn `UserConstructionScript`)