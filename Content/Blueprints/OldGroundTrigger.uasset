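; Ground trigger actor that acts as an actionable, switching on when an actor begins overlapping it and off when one stops.
; Overlaps fire its activated and deactivated dispatchers, which it binds to itself at BeginPlay to swap the static mesh material.
; Each overlap also messages every entry in Receivers through the Receiver interface, printing an error for any that lack it.
; Overlaps are neither filtered nor counted, so any single exit deactivates it.
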(event `self.ReceiveBeginPlay`
  (add `self.OnActivated` (delegate `OnActivated_Event`))
  (add `self.OnDeactivated` (delegate `OnDeactivated_Event`)))

(event `OnDeactivated_Event`
  (`PrimitiveComponent.SetMaterial` (`self.StaticMesh`) 0 "/Engine/EditorMaterials/Cascade/CASC_ModuleDisable_MAT.CASC_ModuleDisable_MAT"))

(event `OnActivated_Event`
  (`KismetSystemLibrary.PrintText` "Material Set")
  (`PrimitiveComponent.SetMaterial` (`self.StaticMesh`) 0 "/Engine/EditorMaterials/CheckMaterial.CheckMaterial"))

(event `self.ReceiveActorBeginOverlap`
  (params (OtherActor :type "Actor Object Reference"))
  (`self.OnActivated`)
  (for _array_element (`self.Receivers`)
    (if (`KismetSystemLibrary.DoesImplementInterface` _array_element "/Game/Blueprints/Interfaces/Receiver.Receiver_C")
      (message `/Game/Blueprints/Interfaces/Receiver.OnSingleActionableActivated` _array_element)
      (else
        (`KismetSystemLibrary.PrintText` "Invalid Receiver Bound To Actionable")))))

(event `self.ReceiveActorEndOverlap`
  (params (OtherActor :type "Actor Object Reference"))
  (`self.OnDeactivated`)
  (for _array_element (`self.Receivers`)
    (if (`KismetSystemLibrary.DoesImplementInterface` _array_element "/Game/Blueprints/Interfaces/Receiver.Receiver_C")
      (message `/Game/Blueprints/Interfaces/Receiver.OnSingleActionableDeactivated` _array_element)
      (else
        (`KismetSystemLibrary.PrintText` "Invalid Receiver Bound To Actionable")))))

(fn `UserConstructionScript`)