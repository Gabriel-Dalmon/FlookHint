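; Grappling gun hook that pulls by shortening the linear limit of a physics constraint while IsPulling is set.
; Each tick wakes the physics object and reduces the limit by a step that grows with the square of pull time, clamped to a maximum speed.
; OnPulled seeds that timer from the object's current velocity and prints it.
; SetLinearLimit sets all three axes to a given size.
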(event `self.ReceiveTick`
  (params (DeltaSeconds :type "Float (single-precision)"))
  (bind _timesincepulling (`self.TimeSincePulling`))
  (if (`self.IsPulling`)
    (set `self.TimeSincePulling` (+ (`self.TimeSincePulling`) DeltaSeconds))
    (`PrimitiveComponent.WakeRigidBody` (`self.PhysicsObject`) "None")
    (bind _returnvalue (`PhysicsConstraintComponent.GetConstraint` (`self.PhysicsConstraint`)))
    (bind (_xmotion _ymotion _zmotion _limit) (`ConstraintInstanceBlueprintLibrary.GetLinearLimits` _returnvalue))
    (`ConstraintInstanceBlueprintLibrary.SetLinearLimits` _returnvalue "LCM_Limited" "LCM_Limited" "LCM_Limited" (- _limit (`KismetMathLibrary.FClamp` (* _timesincepulling _timesincepulling (`self.PullingIncreaseRate`)) 0.1 (`self.MaxPullingSpeed`))))))

(fn `OnPulled`
  (bind _output_get (set `self.TimeSincePulling` (/ (`KismetMathLibrary.VSize` (`SceneComponent.GetComponentVelocity` (`self.PhysicsObject`))) 10.0)))
  (`KismetSystemLibrary.PrintString` (`KismetStringLibrary.Conv_DoubleToString` _output_get)))

(fn `SetLinearLimit`
  (params (LimitSize :type "Float (double-precision)"))
  (`PhysicsConstraintComponent.SetLinearXLimit` (`self.PhysicsConstraint`) "LCM_Limited" LimitSize)
  (`PhysicsConstraintComponent.SetLinearYLimit` (`self.PhysicsConstraint`) "LCM_Limited" LimitSize)
  (`PhysicsConstraintComponent.SetLinearZLimit` (`self.PhysicsConstraint`) "LCM_Limited" LimitSize))

(fn `UserConstructionScript`)