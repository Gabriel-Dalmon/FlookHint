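; BP_ItemPickUp is a pickup actor that hands a carried item to the Cubot character on overlap.
; It spawns its ItemClass actor, attaches it to the character's ItemSocket component, and registers it as the CarriedItem with the character as owner.
; It then adds the gun input mapping context to player controller 0's Enhanced Input subsystem and destroys itself.
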(event `self.ReceiveActorBeginOverlap`
  (params (OtherActor :type "Actor Object Reference"))
  (bind _asbp_cubot_character (cast `/Game/Core/CharacterController/BP_CubotCharacter` OtherActor))
  (bind _returnvalue (`|SpawnActorFromClass` (`self.ItemClass`) (`self.GetLevelTransform`) "AlwaysSpawn" "MultiplyWithRoot" null null))
  (`self.K2_AttachToComponent` _returnvalue (`/Game/Core/CharacterController/BP_CubotCharacter.ItemSocket` _asbp_cubot_character) "None" "KeepRelative" "KeepRelative" "KeepRelative" true)
  (set `/Game/Core/CharacterController/BP_CubotCharacter.CarriedItem` _returnvalue _asbp_cubot_character)
  (`self.SetOwner` _returnvalue _asbp_cubot_character)
  (`EnhancedInputSubsystemInterface.AddMappingContext` (pcsubsystem `EnhancedInputLocalPlayerSubsystem` (`GameplayStatics.GetPlayerController` 0)) "/Game/Inputs/GunInputMapping.GunInputMapping" 0 (struct))
  (`self.K2_DestroyActor`))

(fn `UserConstructionScript`)