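; BP_CubotCharacter is the Cubot character Blueprint that passes player input to the item it carries.
; The shoot and interact Enhanced Input actions call OnInteractBegin on CarriedItem with an enum value, so the item implements the response.
; Shoot picks between two enum values by whether its action value equals one, and interact sends a third.
; Destroying the character also destroys its carried item.
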(event `self.ReceiveDestroyed`
  ; Manage Carried Item
  (`/Engine/EditorBlueprintResources/StandardMacros.IsValid` (`self.CarriedItem`)
    (:`Is Valid`
      (`self.K2_DestroyActor` (`self.CarriedItem`)))))

(event `EnhancedInput|/Game/Inputs/IA_Shoot`
  (params (ActionValue :type "Float (double-precision)") (ElapsedSeconds :type "Float (double-precision)") (TriggeredSeconds :type "Float (double-precision)") (InputAction :type "InputAction Object Reference" :default "/Game/Inputs/IA_Shoot.IA_Shoot"))
  ; Manage Carried Item
  (:`Triggered`
    (`/Engine/EditorBlueprintResources/StandardMacros.IsValid` (`self.CarriedItem`)
      (:`Is Valid`
        (if (!= ActionValue 1.0)
          (`/Game/Blueprints/PortalGun/BP_Item.OnInteractBegin` (`self.CarriedItem`) "NewEnumerator0")
          (else
            (`/Game/Blueprints/PortalGun/BP_Item.OnInteractBegin` (`self.CarriedItem`) "NewEnumerator1")))))))

(event `EnhancedInput|/Game/Inputs/IA_Interact`
  (params (ActionValue :type Boolean) (ElapsedSeconds :type "Float (double-precision)") (TriggeredSeconds :type "Float (double-precision)") (InputAction :type "InputAction Object Reference" :default "/Game/Inputs/IA_Interact.IA_Interact"))
  ; Manage Carried Item
  (:`Triggered`
    (`/Engine/EditorBlueprintResources/StandardMacros.IsValid` (`self.CarriedItem`)
      (:`Is Valid`
        (`/Game/Blueprints/PortalGun/BP_Item.OnInteractBegin` (`self.CarriedItem`) "NewEnumerator2")))))

(fn `UserConstructionScript`)