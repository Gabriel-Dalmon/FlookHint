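; Player controller for the Cubot character that handles player input and death with respawn.
; On BeginPlay it adds the Cubot Enhanced Input mapping context, then routes jump, move, look and interact actions to the player pawn, with interact turning on Cubot's lamp.
; On possession it binds to the Cubot health component's death event, which destroys the pawn and asks BaseGameMode to respawn the player.
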(event `self.ReceiveBeginPlay`
  ;[0.5379 1 0.1754] Initialization
  (`EnhancedInputSubsystemInterface.AddMappingContext` (pcsubsystem `EnhancedInputLocalPlayerSubsystem` self) "/Game/Inputs/CubotInputMappingContext.CubotInputMappingContext" 0 (struct)))

(event `EnhancedInput|/Game/Inputs/Jump`
  (params (ActionValue :type Boolean) (ElapsedSeconds :type "Float (double-precision)") (TriggeredSeconds :type "Float (double-precision)") (InputAction :type "InputAction Object Reference" :default "/Game/Inputs/Jump.Jump"))
  ;[1 1 1] Jump Mapping
  (:`Triggered`
    (bind _ascharacter (cast `Character` (`GameplayStatics.GetPlayerPawn` 0)))
    (`Character.Jump` _ascharacter)))

(event `EnhancedInput|/Game/Inputs/Interact`
  (params (ActionValue :type Boolean) (ElapsedSeconds :type "Float (double-precision)") (TriggeredSeconds :type "Float (double-precision)") (InputAction :type "InputAction Object Reference" :default "/Game/Inputs/Interact.Interact"))
  ;[1 1 1] Interaction2 Mapping
  (:`Triggered`
    (bind _ascubot_character (cast `CubotCharacter` (`GameplayStatics.GetPlayerPawn` 0)))
    (`CubotCharacter.TurnOnLamp` _ascubot_character)))

(event `EnhancedInput|/Game/Inputs/Move`
  (params (ActionValue :type "Vector2D Structure") (ElapsedSeconds :type "Float (double-precision)") (TriggeredSeconds :type "Float (double-precision)") (InputAction :type "InputAction Object Reference" :default "/Game/Inputs/Move.Move"))
  ;[1 1 1] Movement Mapping
  (:`Triggered`
    (bind _ascharacter (cast `Character` (`GameplayStatics.GetPlayerPawn` 0)))
    (`Pawn.AddMovementInput` _ascharacter (`self.GetActorRightVector` _ascharacter) ActionValue_X false)
    (`Pawn.AddMovementInput` _ascharacter (`self.GetActorForwardVector` _ascharacter) ActionValue_Y false)))

(event `EnhancedInput|/Game/Inputs/Look`
  (params (ActionValue :type "Vector2D Structure") (ElapsedSeconds :type "Float (double-precision)") (TriggeredSeconds :type "Float (double-precision)") (InputAction :type "InputAction Object Reference" :default "/Game/Inputs/Look.Look"))
  ;[1 1 1] Look Mapping
  (:`Triggered`
    (bind _ascharacter (cast `Character` (`GameplayStatics.GetPlayerPawn` 0)))
    (`Pawn.AddControllerYawInput` _ascharacter ActionValue_X)
    (`Pawn.AddControllerPitchInput` _ascharacter ActionValue_Y)))

(event `self.ReceivePossess`
  (params (PossessedPawn :type "Pawn Object Reference"))
  ;[1 0.1302 0.1302] Death Logic
  (bind _ascubot_character (cast `CubotCharacter` PossessedPawn))
  (add `HealthComponent.OnDeadEvent` (`CubotCharacter.HealthComponent` _ascubot_character) (delegate `On Character Dead`)))

(event `On Character Dead`
  ;[1 0.1302 0.1302] Death Logic
  (`self.K2_DestroyActor` (`GameplayStatics.GetPlayerPawn` 0))
  (bind _asbase_game_mode (cast `/Game/Blueprints/BaseGameMode` (`GameplayStatics.GetGameMode`)))
  (`/Game/Blueprints/BaseGameMode.Respawn Player_Event` _asbase_game_mode self))

(fn `UserConstructionScript`)