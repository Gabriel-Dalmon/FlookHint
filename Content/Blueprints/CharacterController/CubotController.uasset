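; Player controller for Cubot that turns Enhanced Input actions into commands on the player pawn.
; It adds the Cubot mapping context on BeginPlay, then handles each action by fetching player pawn 0 and casting it.
; Move and Look drive actor-relative movement and yaw/pitch, while Interact calls TurnOnLamp on the CubotCharacter.
; Jump works on any Character; failed Jump or Interact casts print a warning.
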(event `self.ReceiveBeginPlay`
  (`EnhancedInputSubsystemInterface.AddMappingContext` (pcsubsystem `EnhancedInputLocalPlayerSubsystem` self) "/Game/Inputs/CubotInputMappingContext.CubotInputMappingContext" 0 (struct)))

(event `EnhancedInput|/Game/Inputs/Jump`
  (params (ActionValue :type Boolean) (ElapsedSeconds :type "Float (double-precision)") (TriggeredSeconds :type "Float (double-precision)") (InputAction :type "InputAction Object Reference" :default "/Game/Inputs/Jump.Jump"))
  (:`Triggered`
    (bind _ascharacter (cast `Character` (`GameplayStatics.GetPlayerPawn` 0))
      (:`then`
        (`Character.Jump` _ascharacter))
      (:`CastFailed`
        (`KismetSystemLibrary.PrintText` "Non character possessed by cubot controller" true true (struct :`R` 1.0 :`B` 0.154543 :`A` 1.0))))))

(event `EnhancedInput|/Game/Inputs/Interact`
  (params (ActionValue :type Boolean) (ElapsedSeconds :type "Float (double-precision)") (TriggeredSeconds :type "Float (double-precision)") (InputAction :type "InputAction Object Reference" :default "/Game/Inputs/Interact.Interact"))
  (:`Triggered`
    (bind _ascubot_character (cast `CubotCharacter` (`GameplayStatics.GetPlayerPawn` 0))
      (:`then`
        (`CubotCharacter.TurnOnLamp` _ascubot_character))
      (:`CastFailed`
        (`KismetSystemLibrary.PrintText` "Non cubot character possessed by cubot controller" true true (struct :`R` 1.0 :`B` 0.154543 :`A` 1.0))))))

(event `EnhancedInput|/Game/Inputs/Move`
  (params (ActionValue :type "Vector2D Structure") (ElapsedSeconds :type "Float (double-precision)") (TriggeredSeconds :type "Float (double-precision)") (InputAction :type "InputAction Object Reference" :default "/Game/Inputs/Move.Move"))
  (:`Triggered`
    (bind _ascubot_character (cast `CubotCharacter` (`GameplayStatics.GetPlayerPawn` 0)))
    (`Pawn.AddMovementInput` _ascubot_character (`self.GetActorRightVector` _ascubot_character) ActionValue_X false)
    (`Pawn.AddMovementInput` _ascubot_character (`self.GetActorForwardVector` _ascubot_character) ActionValue_Y false)))

(event `EnhancedInput|/Game/Inputs/Look`
  (params (ActionValue :type "Vector2D Structure") (ElapsedSeconds :type "Float (double-precision)") (TriggeredSeconds :type "Float (double-precision)") (InputAction :type "InputAction Object Reference" :default "/Game/Inputs/Look.Look"))
  (:`Triggered`
    (bind _ascubot_character (cast `CubotCharacter` (`GameplayStatics.GetPlayerPawn` 0)))
    (`Pawn.AddControllerYawInput` _ascubot_character ActionValue_X)
    (`Pawn.AddControllerPitchInput` _ascubot_character ActionValue_Y)))

(fn `UserConstructionScript`)