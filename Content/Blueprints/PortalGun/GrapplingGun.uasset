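; Grappling gun that hooks onto a line-traced target and pulls the character toward it.
; Shoot toggles the hook, switching movement between Flying and Falling and showing or hiding the cable.
; Interact starts the pull; Tick updates the cable end and applies force toward the attach point, skewed by movement input.
; The trace returns ImpactNormal as the attach point, and IsActorAttachable's "Attachable" tag check is unconnected.
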(event `Shoot`
  (params (Value :type "Float (double-precision)"))
  (if (`self.IsAttached`)
    (`self.OnHookReleased`)
    (else
      (bind (_attachpoint _attachactor _hasfoundattachpoint) (`self.FindGrapplingPoint`))
      (if (and (`self.IsActorAttachable` _attachactor) _hasfoundattachpoint)
        (set `self.AttachPoint` _attachpoint)
        (`self.OnHookAttached`)))))

(event `Interact`
  (set `self.IsPulling` true))

(event `self.ReceiveTick`
  (params (DeltaSeconds :type "Float (single-precision)"))
  (if (`self.IsAttached`)
    (set `CableComponent.EndLocation` (`KismetMathLibrary.InverseTransformLocation` (`self.GetTransform`) (`self.AttachPoint`)) (`self.Cable`))
    (if (`self.IsPulling`)
      (`CharacterMovementComponent.AddForce` (`Character.CharacterMovement` (`self.CharacterRef`)) (* (`KismetMathLibrary.Normal` (+ (`KismetMathLibrary.GetDirectionUnitVector` (`self.K2_GetActorLocation`) (`self.AttachPoint`)) (* (* (`self.GetActorRightVector`) (`PawnMovementComponent.GetLastInputVector` (`Character.CharacterMovement` (`self.CharacterRef`)))) 0.7))) (`self.PullingForce`))))))

(fn `FindGrapplingPoint`
  (returns (AttachPoint :type "Vector Structure") (AttachActor :type "Actor Object Reference") (HasFoundAttachPoint :type Boolean))
  (bind _muzzle (`self.Muzzle`))
  (bind _returnvalue (`SceneComponent.K2_GetComponentLocation` _muzzle))
  (bind (_outhit _returnvalue_2) (`KismetSystemLibrary.LineTraceSingle` :`Start` _returnvalue :`End` (+ _returnvalue (* (`KismetMathLibrary.GetForwardVector` (`SceneComponent.K2_GetComponentRotation` _muzzle)) (`self.GrapplingRange`))) :`TraceChannel` "TraceTypeQuery1" :`DrawDebugType` "ForDuration"))
  (bind (_bblockinghit _binitialoverlap _time _distance _location _impactpoint _normal _impactnormal _physmat _hitactor) (`GameplayStatics.BreakHitResult` _outhit))
  (return _impactnormal _hitactor _returnvalue_2))

(fn `OnHookAttached`
  (`CharacterMovementComponent.SetMovementMode` (`Character.CharacterMovement` (`self.CharacterRef`)) "MOVE_Flying" 0)
  (`self.OnHookUpdated` true))

(fn `OnHookReleased`
  (`CharacterMovementComponent.SetMovementMode` (`Character.CharacterMovement` (`self.CharacterRef`)) "MOVE_Falling" 0)
  (`self.OnHookUpdated` false)
  (set `self.IsPulling` false))

(fn `OnHookUpdated`
  (params (IsAttached :type Boolean))
  (set `self.IsAttached` IsAttached)
  (`SceneComponent.SetVisibility` (`self.Cable`) IsAttached false))

(fn `UserConstructionScript`)