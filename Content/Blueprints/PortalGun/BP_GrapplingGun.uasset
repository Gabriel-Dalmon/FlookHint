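; Grappling gun that lets its Cubot character owner hook onto actors and pull toward them.
; Primary interaction toggles the hook via a camera-direction trace from the muzzle, switching movement between Flying and Falling and showing the cable.
; While secondary is held, Tick applies force toward AttachPoint, skewed by movement input.
; AttachPoint stores the hit's ImpactNormal rather than its location, and IsActorAttachable's "Attachable" tag check is unconnected.
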(event `self.ReceiveTick`
  (params (DeltaSeconds :type "Float (single-precision)"))
  (if (`self.IsAttached`)
    (set `CableComponent.EndLocation` (`KismetMathLibrary.InverseTransformLocation` (`self.GetTransform`) (`self.AttachPoint`)) (`self.Cable`))
    (if (`self.IsPulling`)
      (bind _ascubot_character (cast `CubotCharacter` (`self.GetOwner`)))
      (bind _charactermovement (`Character.CharacterMovement` _ascubot_character))
      (`CharacterMovementComponent.AddForce` _charactermovement (* (`KismetMathLibrary.Normal` (+ (`KismetMathLibrary.GetDirectionUnitVector` (`self.K2_GetActorLocation`) (`self.AttachPoint`)) (* (* (`self.GetActorRightVector`) (`PawnMovementComponent.GetLastInputVector` _charactermovement)) 0.7))) (`self.PullingForce`))))))

(fn `FindGrapplingPoint`
  (returns (AttachPoint :type "Vector Structure") (AttachActor :type "Actor Object Reference") (HasFoundAttachPoint :type Boolean))
  (bind _returnvalue (`SceneComponent.K2_GetComponentLocation` (`self.Muzzle`)))
  (bind _asbp_cubot_character (cast `/Game/Blueprints/CharacterController/BP_CubotCharacter` (`self.GetOwner`)))
  (bind (_outhit _returnvalue_2) (`KismetSystemLibrary.LineTraceSingle` :`Start` _returnvalue :`End` (+ _returnvalue (* (`KismetMathLibrary.GetForwardVector` (`SceneComponent.K2_GetComponentRotation` (`/Game/Blueprints/CharacterController/BP_CubotCharacter.Camera` _asbp_cubot_character))) (`self.GrapplingRange`))) :`TraceChannel` "TraceTypeQuery1" :`DrawDebugType` "ForDuration"))
  (bind (_bblockinghit _binitialoverlap _time _distance _location _impactpoint _normal _impactnormal _physmat _hitactor) (`GameplayStatics.BreakHitResult` _outhit))
  (return _impactnormal _hitactor _returnvalue_2))

(fn `OnHookAttached`
  (bind _ascubot_character (cast `CubotCharacter` (`self.GetOwner`)))
  (`CharacterMovementComponent.SetMovementMode` (`Character.CharacterMovement` _ascubot_character) "MOVE_Flying" 0)
  (`self.OnHookUpdated` true))

(fn `OnHookReleased`
  (bind _ascubot_character (cast `CubotCharacter` (`self.GetOwner`)))
  (`CharacterMovementComponent.SetMovementMode` (`Character.CharacterMovement` _ascubot_character) "MOVE_Falling" 0)
  (`self.OnHookUpdated` false)
  (set `self.IsPulling` false))

(fn `OnHookUpdated`
  (params (IsAttached :type Boolean))
  (set `self.IsAttached` IsAttached)
  (`SceneComponent.SetVisibility` (`self.Cable`) IsAttached false))

(fn `OnInteractBegin`
  (params (InteractionType :type "/Game/InteractionTypes Enum" :default "NewEnumerator0"))
  (`parent.OnInteractBegin` InteractionType)
  (switch `/Game/InteractionTypes` InteractionType
    (:`NewEnumerator0`
      (if (`self.IsAttached`)
        (`self.OnHookReleased`)
        (else
          (`self.TryAttachHook`))))
    (:`NewEnumerator1`
      (if (`self.IsAttached`)
        (set `self.IsPulling` true)))))

(fn `OnInteractEnd`
  (params (InteractionType :type "/Game/InteractionTypes Enum" :default "NewEnumerator0"))
  (`parent.OnInteractEnd` InteractionType)
  (switch `/Game/InteractionTypes` InteractionType
    (:`NewEnumerator1`
      (if (`self.IsAttached`)
        (set `self.IsPulling` false)))))

(fn `TryAttachHook`
  (bind (_attachpoint _attachactor _hasfoundattachpoint) (`self.FindGrapplingPoint`))
  (if (and (`self.IsActorAttachable` _attachactor) _hasfoundattachpoint)
    (set `self.AttachPoint` _attachpoint)
    (`self.OnHookAttached`)))

(fn `UserConstructionScript`)