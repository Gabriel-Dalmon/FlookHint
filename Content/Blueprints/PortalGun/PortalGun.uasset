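; Portal gun held by BP_CubotCharacter that places two linked, color-coded portals and carries companion cubes.
; On BeginPlay it spawns and links both portals off-map, then destroys them with itself.
; Primary and secondary shots camera-trace for "Placable" actors, move a portal there, banish its overlapping twin, and activate both only within maximum separation.
; Ternary interaction attaches a traced cube to the muzzle socket or releases it, blocking shots while carried.
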(event Custom|ResetPortals
  (Transformation|SetActorLocation (Utilities|Array|Get(acopy) (Variables|Default|GetPortals)) "-1000.000000,-1000.000000,-10000.000000" false true)
  (Transformation|SetActorLocation (Utilities|Array|Get(acopy) (Variables|Default|GetPortals) 1) "-1000.000000,-1000.000000,-10000.000000" false true))

(event EventBeginPlay
  (CallFunction|InitializePortals))

(event EventTick
  (params (DeltaSeconds :type Float%20%28single-precision%29)))

(event EventDestroyed
  (CallFunction|DestroyPortals))

(fn ConstructionScript)

(fn InitializePortals
  ;[1 1 1] Spawn Portals
  (bind _return_value (CallFunction|InstanciatePortal "(R=0.527115,G=0.323143,B=0.051269,A=1.000000)"))
  (bind _return_value_2 (CallFunction|InstanciatePortal "(R=0.006995,G=0.012983,B=0.552012,A=1.000000)"))
  (Utilities|FlowControl|Sequence
    (:then_0
      ;[1 1 1] Link Portals
      (Variables|/Game/Blueprints/Portals/Portal.Portal_C|SetLinkedPortal _return_value _return_value_2))
    (:then_1
      (Variables|/Game/Blueprints/Portals/Portal.Portal_C|SetLinkedPortal _return_value_2 _return_value))
    (:then_2
      (Default|OnLinked _return_value)
      (Default|OnLinked _return_value_2))
    (:then_3
      ;[1 1 1] Store Portals Ref
      (Variables|Default|SetPortals (Utilities|Array|MakeArray _return_value_2 _return_value)))))

(fn InstanciatePortal
  (params (Color :type Linear%20Color%20Structure))
  (bind _returnvalue (Game|SpawnActorfromClass "/Game/Blueprints/Portals/Portal.Portal_C" (Math|Transform|MakeTransform "-10000.000000,-10000.000000,-10000.000000") "Undefined" "MultiplyWithRoot" 0 0))
  (Rendering|Material|SetVectorParameterValue (Variables|/Game/Blueprints/Portals/Portal.Portal_C|GetPortalMaterial _returnvalue) "BorderColor" Color :!class /Script/Engine.MaterialInstanceDynamic)
  (return _returnvalue))

(fn DestroyPortals
  (for _array_element (Variables|Default|GetPortals)
    (Actor|DestroyActor _array_element)))

(fn OnInteractBegin
  (params (InteractionType :type InteractionTypes%20Enum :default "NewEnumerator0"))
  (|CallParentFunction InteractionType)
  (switch Utilities|FlowControl|Switch|SwitchonInteractionTypes InteractionType
    (:NewEnumerator0
      (CallFunction|OnShot 0.0))
    (:NewEnumerator1
      (CallFunction|OnShot 1.0))
    (:NewEnumerator2
      (CallFunction|OnPickedUp))))

(fn OnShot
  (params (Value :type Float%20%28double-precision%29))
  (bind _muzzle (Variables|Default|GetMuzzle))
  (if (Utilities|IsValid (Variables|Default|GetCompanion))
    (Development|PrintString "Can't shoot on your companion!!")
    (else
      (if (== Value 1.0)
        (Effects|Components|ParticleSystem|SetColorParameter _muzzle "Color" "(R=0.078431,G=0.117647,B=0.764706,A=1.000000)")
        (else
          (Effects|Components|ParticleSystem|SetColorParameter _muzzle "Color" "(R=0.529412,G=0.321569,B=0.050980,A=1.000000)")))
      (Components|Activation|Activate _muzzle false)
      (bind _asbp_cubot_character (Utilities|Casting|CastToBP_CubotCharacter (Components|GetOwner)))
      (bind (_outhit _returnvalue) (Collision|LineTraceByChannel (Transformation|GetWorldLocation (Variables|/Game/Blueprints/CharacterController/BP_CubotCharacter.BP_CubotCharacter_C|GetCamera _asbp_cubot_character)) (+ (Transformation|GetWorldLocation (Variables|/Game/Blueprints/CharacterController/BP_CubotCharacter.BP_CubotCharacter_C|GetCamera _asbp_cubot_character)) (* (Math|Vector|GetForwardVector (Transformation|GetWorldRotation (Variables|/Game/Blueprints/CharacterController/BP_CubotCharacter.BP_CubotCharacter_C|GetCamera _asbp_cubot_character))) (|20000))) "TraceTypeQuery1" false (Variables|Default|GetPortals) "None"))
      (if _returnvalue
        (if (Actor|ActorHasTag (.HitActor (Collision|BreakHitResult _outhit)) "Placable")
          (if (== Value 1.0)
            (Development|PrintString "1")
            (if (<= (Math|Vector|Distance(Vector) (Transformation|GetActorLocation (Utilities|Array|Get(acopy) (Variables|Default|GetPortals) 1)) (+ (.ImpactPoint (Collision|BreakHitResult _outhit)) (.Normal (Collision|BreakHitResult _outhit)))) 3e+02)
              (Transformation|SetActorLocation (Utilities|Array|Get(acopy) (Variables|Default|GetPortals) 1) "-1000.000000,-1000.000000,-10000.000000" false true))
            (Transformation|SetActorLocation (Utilities|Array|Get(acopy) (Variables|Default|GetPortals)) (+ (.ImpactPoint (Collision|BreakHitResult _outhit)) (.Normal (Collision|BreakHitResult _outhit))) false false)
            (Transformation|SetActorRotation (Utilities|Array|Get(acopy) (Variables|Default|GetPortals)) (Math|Conversions|RotationFromXVector (.Normal (Collision|BreakHitResult _outhit))) true)
            (else
              (Development|PrintString "2")
              (if (<= (Math|Vector|Distance(Vector) (Transformation|GetActorLocation (Utilities|Array|Get(acopy) (Variables|Default|GetPortals))) (+ (.ImpactPoint (Collision|BreakHitResult _outhit)) (.Normal (Collision|BreakHitResult _outhit)))) 3e+02)
                (Transformation|SetActorLocation (Utilities|Array|Get(acopy) (Variables|Default|GetPortals)) "-1000.000000,-1000.000000,-10000.000000" false true))
              (Transformation|SetActorLocation (Utilities|Array|Get(acopy) (Variables|Default|GetPortals) 1) (+ (.ImpactPoint (Collision|BreakHitResult _outhit)) (.Normal (Collision|BreakHitResult _outhit))) false false)
              (Transformation|SetActorRotation (Utilities|Array|Get(acopy) (Variables|Default|GetPortals) 1) (Math|Conversions|RotationFromXVector (.Normal (Collision|BreakHitResult _outhit))) true)))
          (if (<= (Math|Vector|Distance(Vector) (Transformation|GetActorLocation (Utilities|Array|Get(acopy) (Variables|Default|GetPortals))) (Transformation|GetActorLocation (Utilities|Array|Get(acopy) (Variables|Default|GetPortals) 1))) (* (Variables|Default|GetMaxDistanceBetweenPortalsInMeters) 1e+02))
            (Default|SetActivation (Utilities|Array|Get(acopy) (Variables|Default|GetPortals)) true)
            (Default|SetActivation (Utilities|Array|Get(acopy) (Variables|Default|GetPortals) 1) true)
            (else
              (Default|SetActivation (Utilities|Array|Get(acopy) (Variables|Default|GetPortals)) false)
              (Default|SetActivation (Utilities|Array|Get(acopy) (Variables|Default|GetPortals) 1) false)))
          (else
            (Development|PrintString "Non placable wall")))
        (else
          (Development|PrintString "Didn't hit"))))))

(fn OnPickedUp
  (bind _portalgun (Variables|Default|GetportalGun))
  (bind _asbp_cubot_character (Utilities|Casting|CastToBP_CubotCharacter (Components|GetOwner)))
  (if (Utilities|IsValid (Variables|Default|GetCompanion))
    (Physics|SetSimulatePhysics (Variables|/Game/Blueprints/BP_CompanionCube.BP_CompanionCube_C|GetcubeCompanion (Variables|Default|GetCompanion)) true)
    (Transformation|DetachFromComponent (Variables|/Game/Blueprints/BP_CompanionCube.BP_CompanionCube_C|GetcubeCompanion (Variables|Default|GetCompanion)) "KeepWorld" "KeepWorld" "KeepWorld" true)
    (Collision|SetCollisionEnabled (Variables|/Game/Blueprints/BP_CompanionCube.BP_CompanionCube_C|GetcubeCompanion (Variables|Default|GetCompanion)) (Variables|Default|GetCarriedObjectCollisionsType))
    (Physics|SetPhysicsLinearVelocity (Variables|/Game/Blueprints/BP_CompanionCube.BP_CompanionCube_C|GetcubeCompanion (Variables|Default|GetCompanion)) (Variables|/Script/Engine.MovementComponent|GetVelocity (Pawn|GetMovementComponent (Game|GetPlayerCharacter 0))) false "None")
    (Variables|Default|SetCompanion 0)
    (Components|Timeline|SetPlayRate _portalgun -1.0)
    (Audio|Components|Audio|Play _portalgun false)
    (else
      (bind (_outhit _returnvalue) (Collision|LineTraceByChannel (Transformation|GetWorldLocation (Variables|/Game/Blueprints/CharacterController/BP_CubotCharacter.BP_CubotCharacter_C|GetCamera _asbp_cubot_character)) (+ (Transformation|GetWorldLocation (Variables|/Game/Blueprints/CharacterController/BP_CubotCharacter.BP_CubotCharacter_C|GetCamera _asbp_cubot_character)) (* (Math|Vector|GetForwardVector (Transformation|GetWorldRotation (Variables|/Game/Blueprints/CharacterController/BP_CubotCharacter.BP_CubotCharacter_C|GetCamera _asbp_cubot_character))) (|800))) "TraceTypeQuery1" false 0 "None"))
      (if _returnvalue
        (bind _asbp_companion_cube (Utilities|Casting|CastToBP_CompanionCube (.HitActor (Collision|BreakHitResult _outhit)))
          (:then
            (bind _output_get (Variables|Default|SetCompanion _asbp_companion_cube))
            (Variables|Default|SetCarriedObjectCollisionsType (Collision|GetCollisionEnabled (Variables|/Game/Blueprints/BP_CompanionCube.BP_CompanionCube_C|GetcubeCompanion _output_get)))
            (Physics|SetSimulatePhysics (Variables|/Game/Blueprints/BP_CompanionCube.BP_CompanionCube_C|GetcubeCompanion _output_get) false)
            (Collision|SetCollisionEnabled (Variables|/Game/Blueprints/BP_CompanionCube.BP_CompanionCube_C|GetcubeCompanion _output_get) "NoCollision")
            (Transformation|AttachComponentToComponent _output_get (Variables|Default|GetportalGunChassis) "Canon" "SnapToTarget" "KeepRelative" "KeepWorld" true)
            (Components|Animation|PlayAnimation (Variables|Default|GetportalGun) "/Game/Animations/portalGun_Skeleton_Sequence.portalGun_Skeleton_Sequence" false))
          (:CastFailed
            (Development|PrintString "Are you cheating on your companion?!!")))
        (else
          (Development|PrintString "Didn't hit"))))))