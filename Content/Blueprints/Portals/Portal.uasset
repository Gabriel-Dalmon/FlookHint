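; Portal actor that shows its linked portal's camera view and teleports overlapping actors to that portal's spawn point while active.
; On BeginPlay it creates a viewport-sized render target, fed by the linked portal's camera and displayed through a dynamic material, replaced by a cross when deactivated.
; Controlled pawns set player 0's view and carry velocity through, flipped in portal-local space; other actors just take the exit rotation.
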(event `self.ReceiveBeginPlay`
  (bind (_returnvalue_x _returnvalue_y) (`KismetMathLibrary.BreakVector2D` (`WidgetLayoutLibrary.GetViewportSize`)))
  (bind _returnvalue (`KismetMaterialLibrary.CreateDynamicMaterialInstance` "/Game/Blueprints/Portals/RenderMaterial.RenderMaterial"))
  (bind _output_get (set `self.PortalMaterial` _returnvalue))
  (`PrimitiveComponent.SetMaterial` (`self.RenderSurface`) 0 _output_get)
  (bind _returnvalue_2 (`KismetRenderingLibrary.CreateRenderTarget2D` (`KismetMathLibrary.FTrunc` _returnvalue_x) (`KismetMathLibrary.FTrunc` _returnvalue_y)))
  (bind _output_get_2 (set `self.RenderTexture` _returnvalue_2))
  (`MaterialInstanceDynamic.SetTextureParameterValue` (`self.PortalMaterial`) "Texture" _output_get_2)
  (set `SceneCaptureComponent2D.TextureTarget` (`self.RenderTexture`) (`/Game/Blueprints/Portals/Portal.RenderCamera` (`self.LinkedPortal`)))
  (add `self.SetActivationState` (delegate `SetActivation`)))

(event `SetActivation` :!signature `self.SetActivationState`
  (params (NewActivationState :type Boolean))
  (bind _output_get (set `self.ActivationState` NewActivationState))
  (if _output_get
    (`MaterialInstanceDynamic.SetTextureParameterValue` (`self.PortalMaterial`) "Texture" (`self.RenderTexture`))
    (else
      (`MaterialInstanceDynamic.SetTextureParameterValue` (`self.PortalMaterial`) "Texture" "/Game/Blueprints/Portals/cross.cross"))))

(event `self.ReceiveActorBeginOverlap`
  (params (OtherActor :type "Actor Object Reference"))
  (bind _returnvalue (`Pawn.GetMovementComponent` (`GameplayStatics.GetPlayerCharacter` 0)))
  (bind _returnvalue_2 (`SceneComponent.K2_GetComponentRotation` (`/Game/Blueprints/Portals/Portal.LookDirection` (`self.LinkedPortal`))))
  (if (`self.ActivationState`)
    (cast `/Game/Blueprints/Portals/Portal` OtherActor
      (:`then`
        (`KismetSystemLibrary.PrintString` "overlapping portals"))
      (:`CastFailed`
        (`self.K2_SetActorLocation` OtherActor (`SceneComponent.K2_GetComponentLocation` (`/Game/Blueprints/Portals/Portal.SpawnPoint` (`self.LinkedPortal`))) false true)
        (bind _aspawn (cast `Pawn` OtherActor)
          (:`then`
            (if (`Pawn.IsControlled` _aspawn)
              (`Controller.SetControlRotation` (`GameplayStatics.GetPlayerController` 0) _returnvalue_2)
              (bind _newparam (`self.UpdateVelocity` (`MovementComponent.Velocity` _returnvalue)))
              (set `MovementComponent.Velocity` _newparam _returnvalue)
              (else
                (`self.K2_SetActorRotation` OtherActor _returnvalue_2 true))))
          (:`CastFailed`
            (`self.K2_SetActorRotation` OtherActor _returnvalue_2 true)))))))

(fn `UpdateVelocity`
  (params (Velocity :type "Vector Structure"))
  (returns (NewParam :type "Vector Structure"))
  (return (* (`KismetMathLibrary.TransformDirection` (`self.GetTransform` (`self.LinkedPortal`)) (`KismetMathLibrary.MirrorVectorByNormal` (`KismetMathLibrary.MirrorVectorByNormal` (`KismetMathLibrary.InverseTransformDirection` (`self.GetTransform`) (`KismetMathLibrary.Normal` Velocity)) (1.0 0.0 0.0)) (0.0 1.0 0.0))) (`KismetMathLibrary.VSize` (`local.Velocity`)))))

(fn `UserConstructionScript`)